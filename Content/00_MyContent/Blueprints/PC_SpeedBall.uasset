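; Player controller for a ball-rolling game that turns movement input into spin on the player's ball.
; The MoveForward and MoveRight axes each call a helper that gets the ball component from the controlled pawn through GetBallMessage.
; If the component is valid, the helper adds Speed-scaled torque as an acceleration change, forward on Y and right on X, so physics does the rolling.
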(event `InputAxis|MoveForward`
  (params (AxisValue :type "Float (single-precision)"))
  ;[0.7763 0.2317 1] Player Controller
  (`self.ApplyBallMoveForward` AxisValue (`GameplayStatics.GetPlayerPawn` 0)))

(event `InputAxis|MoveRight`
  (params (AxisValue :type "Float (single-precision)"))
  ;[0.7763 0.2317 1] Player Controller
  (`self.ApplyBallMoveRight` AxisValue (`GameplayStatics.GetPlayerPawn` 0)))

(fn `UserConstructionScript`)