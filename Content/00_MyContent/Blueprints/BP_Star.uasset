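; BP_Star is a collectible star that bobs on a looping timeline and awards a point when the player touches it.
; A one-shot overlap on the collision sphere checks the Player tag, adds a star through the game mode's message interface and plays a sound.
; Looting hides the particles, raises and spins the actor with a second timeline, then destroys it.
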(event `self.ReceiveBeginPlay`
  ;[0.3816 0.4086 1] Star Idle Animation Movement
  (bind (_direction _looplocationz) (`Timeline|StarMovement`)
    (:`Update`
      (`SceneComponent.K2_SetRelativeLocation` (`self.Star`) (`KismetMathLibrary.MakeVector` 0.0 0.0 _looplocationz) false false))))

(event `self.CollisionSphere.OnComponentBeginOverlap`
  (params (OverlappedComponent :type "PrimitiveComponent Object Reference") (OtherActor :type "Actor Object Reference") (OtherComp :type "PrimitiveComponent Object Reference") (OtherBodyIndex :type Integer) (bFromSweep :type Boolean) (SweepResult :type "HitResult Structure (by ref)"))
  ;[1 0.8917 0.4541] Add Star Point
  (if (not (`self.HasAlreadyCollided`))
    (set `self.HasAlreadyCollided` true)
    (if (`self.ActorHasTag` OtherActor "Player")
      (bind _gamemodespeedball (message `/Game/00_MyContent/Blueprints/Interfaces/INT_GMSpeedBall.GetGameModeSpeedBall` (`GameplayStatics.GetGameMode`)))
      (`/Game/00_MyContent/Blueprints/GM_SpeedBall.AddStar` _gamemodespeedball)
      (`GameplayStatics.PlaySound2D` "/Game/00_MyContent/Audio/SoundCues/SC_Star.SC_Star" 1.0 1.0 0.0 null null)
      (`self.Star Looted`))))

(event `Star Looted`
  (bind (_returnvalue_roll _returnvalue_pitch _returnvalue_yaw) (`KismetMathLibrary.BreakRotator` (`self.K2_GetActorRotation`)))
  (bind (_returnvalue_x _returnvalue_y _returnvalue_z) (`KismetMathLibrary.BreakVector` (`self.K2_GetActorLocation`)))
  ;[1 0.3434 0.3633] Star Loot Animation And Destroy On Finish
  (`SceneComponent.SetVisibility` (`self.P_Star`) false false) ; Disable particle system visibility on animation start
  (bind (_direction _updatelocation _updaterotation) (`Timeline|StarLootMovement`)
    (:`Update`
      (`self.K2_SetActorRelativeLocation` (`KismetMathLibrary.MakeVector` _returnvalue_x _returnvalue_y (+ _returnvalue_z (.z _updatelocation))))
      (`self.K2_SetActorRelativeRotation` (`KismetMathLibrary.MakeRotator` _returnvalue_roll _returnvalue_pitch (+ (.z _updaterotation) _returnvalue_yaw))))
    (:`Finished`
      (`self.K2_DestroyActor`))))

(fn `UserConstructionScript`)